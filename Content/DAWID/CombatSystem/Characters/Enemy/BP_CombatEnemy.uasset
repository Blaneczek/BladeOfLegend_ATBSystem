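; BP_CombatEnemy is an enemy character for the combat system that shows damage and status feedback through widget components.
; On BeginPlay, after a short delay, it applies the combat animation class to its animation component, falling back to the wolf combat AnimBP if none is valid.
; Events forward damage, heal, element and dodge data to the damage display widget, and add or remove statuses on the status widget.
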(event `self.ReceiveBeginPlay`
  (bind _returnvalue (`self.GetCombatAnimClass`))
  (`parent.ReceiveBeginPlay`)
  (`KismetSystemLibrary.Delay` 0.2)
  (if (`KismetSystemLibrary.IsValidClass` _returnvalue)
    (`PaperZDAnimationComponent.SetAnimInstanceClass` (`self.AnimationComponent`) _returnvalue)
    (else
      (`PaperZDAnimationComponent.SetAnimInstanceClass` (`self.AnimationComponent`) "/Game/Blueprints/Animations/Wolf/ABP_Wolf_Combat.ABP_Wolf_Combat_C"))))

(event `self.DisplayTextDMG`
  (params (DMG :type "Float (single-precision)") (bHeal :type Boolean) (DMGElement :type "ECombatElementType Enum" :default "FIRE") (bDodge :type Boolean))
  (bind _aswbp_dmgdisplay (cast `/Game/DAWID/CombatSystem/UI/Gameplay/WBP_DMGDisplay` (`WidgetComponent.GetWidget` (`self.DMGDisplay`))))
  (`/Engine/EditorBlueprintResources/StandardMacros.IsValid` _aswbp_dmgdisplay
    (:`Is Valid`
      (`/Game/DAWID/CombatSystem/UI/Gameplay/WBP_DMGDisplay.Set Value` _aswbp_dmgdisplay DMG bHeal DMGElement bDodge))))

(event `self.SetStatusDisplayVisibility`
  (params (Status :type "ECombatStatusType Enum" :default "NONE") (bNewVisibility :type Boolean))
  (bind _aswbp_statuses (cast `/Game/DAWID/CombatSystem/UI/Gameplay/WBP_Statuses` (`WidgetComponent.GetWidget` (`self.StatusDisplay`))))
  (`/Engine/EditorBlueprintResources/StandardMacros.IsValid` _aswbp_statuses
    (:`Is Valid`
      (if bNewVisibility
        (`/Game/DAWID/CombatSystem/UI/Gameplay/WBP_Statuses.Add Status` _aswbp_statuses Status)
        (else
          (`/Game/DAWID/CombatSystem/UI/Gameplay/WBP_Statuses.RemoveStatus` _aswbp_statuses Status))))))

(fn `UserConstructionScript`)