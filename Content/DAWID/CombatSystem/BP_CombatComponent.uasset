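; Combat component that randomly builds the enemy team for a fight based on a difficulty level from 1 to 4.
; GenerateData rolls enemy count, level and type per difficulty, then pulls stats from per-type level maps and assigns sprite, animations and actions.
; Each enemy feeds a shared creation step that totals Exp and gold, before CombatData receives the team.
; BeginPlay passes difficulty 0, which matches no case and generates no enemies.
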(event `self.ReceiveBeginPlay`
  (`self.Generate Data` 0))

(fn `Generate Data`
  (params (DifficultyLevel :type Integer))
  (locals (NumberOfEnemies :type Integer) (EnemiesTypeLevel1 :type "Array of /Game/DAWID/CombatSystem/Data/EEnemyType Enum") (EnemiesTypeLevel2 :type "Array of /Game/DAWID/CombatSystem/Data/EEnemyType Enum") (EnemiesTypeLevel3 :type "Array of /Game/DAWID/CombatSystem/Data/EEnemyType Enum") (EnemiesTypeLevel4 :type "Array of /Game/DAWID/CombatSystem/Data/EEnemyType Enum") (EnemyData :type "Array of EnemyAssetInfo Structure") (Sprite :type "PaperFlipbook Object Reference") (EnemyElement :type "ECombatElementType Enum") (WeaponElement :type "ECombatElementType Enum") (WeaponStatus :type "CombatStatus Structure") (AnimClass :type "PaperZDAnimInstance Class Reference") (TakeDMGAnim :type "PaperZDAnimSequence Object Reference") (TakeDMGSound :type "SoundBase Object Reference") (DeathSound :type "SoundBase Object Reference") (Actions :type "Array of BLAction Soft Class Reference") (Name :type String) (EnemyLvl :type Integer :default 1) (LevelData :type "EnemyLevelData Structure") (StatusesImmunity :type "Set of ECombatStatusType Enum"))
  (bind (_combatdata_combatmap _combatdata_enemydata) (break `CombatData` (`self.CombatData`)))
  (bind (_combatdata_combatmap_2 _combatdata_enemydata_2) (break `CombatData` (`self.CombatData`)))
  (bind (_combatdata_combatmap_3 _combatdata_enemydata_3) (break `CombatData` (`self.CombatData`)))
  (bind (_combatdata_combatmap_4 _combatdata_enemydata_4) (break `CombatData` (`self.CombatData`)))
  (bind (_strength _agility _wisdom _endurance _basehp _baseme _baseattackdmg _basedefense _cooldown _exp _money) (break `EnemyLevelData` (`local.LevelData`)))
  (bind _output_get (set `self.DifficultyLevel` DifficultyLevel))
  (switch `int` _output_get
    (:`1`
      ;[1 1 1] Random number of enemies (Ranges)
      (bind _output_get_2 (set `local.NumberOfEnemies` (`KismetMathLibrary.RandomIntegerInRange` 1 4)))
      (for _ (range _output_get_2)
        ;[1 1 1] Random enemy level (Ranges)
        (set `local.EnemyLvl` (`KismetMathLibrary.RandomIntegerInRange` 1 3))
        ;[1 0.4657 0.1578] On level 1 only wolves and (szczury jak beda)
        (switch `/Game/DAWID/CombatSystem/Data/EEnemyType` (`KismetArrayLibrary.Array_Random` (`local.EnemiesTypeLevel1`))
          (:`NewEnumerator2`
            ;[0.3154 1 0.3934] Wolf
            (set `local.LevelData` (`BlueprintMapLibrary.Map_Find` (`self.Rats`) (`local.EnemyLvl`)))
            (set `local.Sprite` "/Game/PaperAssets/Characters/Rat/FB_Rat_Idle_Right.FB_Rat_Idle_Right")
            ;[1 0.05107 0.7825] OPTIONAL
            (set `local.EnemyElement` "NONE")
            (set `local.WeaponElement` "NONE")
            (set `local.WeaponStatus` (make `CombatStatus` "NONE"))
            (set `local.StatusesImmunity` (`|MakeSet` "NONE" :!type "ECombatStatusType Enum"))
            (set `local.AnimClass` "/Game/Blueprints/Animations/Rat/ABP_Rat.ABP_Rat_C")
            (set `local.TakeDMGAnim` "/Game/Blueprints/Animations/Rat/AnimSequences/Rat_Hit_Right.Rat_Hit_Right")
            (set `local.Actions` (`|MakeArray` "/Game/DAWID/CombatSystem/Data/Actions/Rat/Rat_Special.Rat_Special_C" "/Game/DAWID/CombatSystem/Data/Actions/Rat/Rad_DefaultAttack.Rad_DefaultAttack_C" :!type "BLAction Soft Class Reference"))
            (set `local.Name` "Rat"))
          (:`NewEnumerator0`
            ;[0.3154 1 0.3934] Wolf
            (set `local.LevelData` (`BlueprintMapLibrary.Map_Find` (`self.Wolves`) (`local.EnemyLvl`)) :!label _label)
            (set `local.Sprite` "/Game/PaperAssets/Characters/Wolf/FB_Wolf_Attack_Right.FB_Wolf_Attack_Right")
            (set `local.EnemyElement` "NONE")
            (set `local.WeaponElement` "NONE")
            (set `local.WeaponStatus` (make `CombatStatus` "NONE"))
            (set `local.StatusesImmunity` (`|MakeSet` "NONE" :!type "ECombatStatusType Enum"))
            (set `local.AnimClass` "/Game/Blueprints/Animations/Wolf/ABP_Wolf_Combat.ABP_Wolf_Combat_C")
            (set `local.TakeDMGAnim` "/Game/Blueprints/Animations/Wolf/AnimSequences/Wolf_TakeDMG_Right.Wolf_TakeDMG_Right")
            (set `local.Actions` (`|MakeArray` "/Game/DAWID/CombatSystem/Data/Actions/Wolf/Wolf_DefaultAttack.Wolf_DefaultAttack_C" :!type "BLAction Soft Class Reference"))
            (set `local.Name` "Wolf")))
        (bind _returnvalue (`BLEnemyDataAsset.CreateEnemyData` (`.EnemyData` (break `CombatData` (`self.CombatData`))) (`local.EnemyLvl`) (`local.Name`) "/Game/DAWID/CombatSystem/Characters/Enemy/BP_CombatEnemy.BP_CombatEnemy_C" (`local.LevelData`) (`local.EnemyElement`) (`local.WeaponElement`) (`local.StatusesImmunity`) (`local.WeaponStatus`) (`local.Sprite`) (`local.AnimClass`) (`local.TakeDMGAnim`) :!label _label_2))
        (bind (_name _class _maxhp) (break `CombatCharData` _returnvalue))
        (`KismetSystemLibrary.PrintText` (`|FormatText` "{Name}: {HP}" _name _maxhp) true true (struct :`G` 0.66 :`B` 1.0 :`A` 1.0) 1000.0)
        (`KismetArrayLibrary.Array_Add` (`local.EnemyData`) (make `EnemyAssetInfo` (`local.EnemyLvl`) _returnvalue (`local.Actions`)))
        (`self.AddExpAndGold` _exp _money))
      (`BLEnemyDataAsset.SetEnemyTeamData` _combatdata_enemydata_3 (`local.EnemyData`)))
    (:`2`
      (bind _output_get_3 (set `local.NumberOfEnemies` (`KismetMathLibrary.RandomIntegerInRange` 5 9)))
      (for _ (range _output_get_3)
        (set `local.EnemyLvl` (`KismetMathLibrary.RandomIntegerInRange` 3 6))
        ;[1 0.4657 0.1578] On level 2 only wolves and (szczury jak beda) and golbins
        (switch `/Game/DAWID/CombatSystem/Data/EEnemyType` (`KismetArrayLibrary.Array_Random` (`local.EnemiesTypeLevel2`))
          (:`NewEnumerator0`
            (goto _label))
          (:`NewEnumerator1`
            ;[1 0.8591 0.2111] Golbin
            (set `local.LevelData` (`BlueprintMapLibrary.Map_Find` (`self.Golbins`) (`local.EnemyLvl`)) :!label _label_3)
            (set `local.Sprite` "/Game/PaperAssets/Characters/Goblin/FB_Goblin_Attack1_Right.FB_Goblin_Attack1_Right")
            (set `local.EnemyElement` "NONE")
            (set `local.WeaponElement` "NONE")
            (set `local.WeaponStatus` (make `CombatStatus` "NONE"))
            (set `local.StatusesImmunity` (`|MakeSet` "NONE" :!type "ECombatStatusType Enum"))
            (set `local.AnimClass` "/Game/Blueprints/Animations/Goblin/ABP_Goblin.ABP_Goblin_C")
            (set `local.TakeDMGAnim` "/Game/Blueprints/Animations/Goblin/AnimSequences/Goblin_TakeDMG.Goblin_TakeDMG")
            (set `local.Actions` (`|MakeArray` "/Game/DAWID/CombatSystem/Data/Actions/Goblin/Goblin_DefaultAttack.Goblin_DefaultAttack_C" "/Game/DAWID/CombatSystem/Data/Actions/Goblin/Goblin_SpecialAttack2.Goblin_SpecialAttack2_C" "/Game/DAWID/CombatSystem/Data/Actions/Goblin/Goblin_ThrowKnife.Goblin_ThrowKnife_C" :!type "BLAction Soft Class Reference"))
            (set `local.Name` "Golbin")
            (goto _label_2))))
      (`BLEnemyDataAsset.SetEnemyTeamData` _combatdata_enemydata_4 (`local.EnemyData`)))
    (:`3`
      (bind _output_get_4 (set `local.NumberOfEnemies` (`KismetMathLibrary.RandomIntegerInRange` 3 6)))
      (for _ (range _output_get_4)
        (set `local.EnemyLvl` (`KismetMathLibrary.RandomIntegerInRange` 7 10))
        ;[1 0.4657 0.1578] On level 3 only golbins and werewolves and (jakis jeszcze)
        (switch `/Game/DAWID/CombatSystem/Data/EEnemyType` (`KismetArrayLibrary.Array_Random` (`local.EnemiesTypeLevel3`))
          (:`NewEnumerator1`
            (goto _label_3))
          (:`NewEnumerator3`
            ;[0.4669 0.4693 1] Werewolf
            (set `local.LevelData` (`BlueprintMapLibrary.Map_Find` (`self.Werewolf`) (`local.EnemyLvl`)))
            (set `local.Sprite` "/Game/PaperAssets/Characters/Werewolf/Grey/FB_Werewolf_Grey_Atk1_Right.FB_Werewolf_Grey_Atk1_Right")
            (set `local.EnemyElement` "NONE")
            (set `local.WeaponElement` "NONE")
            (set `local.WeaponStatus` (make `CombatStatus` "NONE"))
            (set `local.StatusesImmunity` (`|MakeSet` "NONE" :!type "ECombatStatusType Enum"))
            (set `local.AnimClass` "/Game/Blueprints/Animations/Werewolf/Grey/ABP_Werewolf_Grey.ABP_Werewolf_Grey_C")
            (set `local.TakeDMGAnim` "/Game/Blueprints/Animations/Werewolf/Grey/AnimSequences/Werewolf_Grey_Hit_Right.Werewolf_Grey_Hit_Right")
            (set `local.Actions` (`|MakeArray` "/Game/DAWID/CombatSystem/Data/Actions/Werewolf/Werewolf_DefaultAttack.Werewolf_DefaultAttack_C" "/Game/DAWID/CombatSystem/Data/Actions/Werewolf/Werewolf_SpecialAttack.Werewolf_SpecialAttack_C" :!type "BLAction Soft Class Reference"))
            (set `local.Name` "Werewolf")
            (goto _label_2))))
      (`BLEnemyDataAsset.SetEnemyTeamData` _combatdata_enemydata_2 (`local.EnemyData`)))
    (:`4`
      (bind _output_get_5 (set `local.NumberOfEnemies` (`KismetMathLibrary.RandomIntegerInRange` 3 6)))
      (for _ (range _output_get_5)
        (set `local.EnemyLvl` (`KismetMathLibrary.RandomIntegerInRange` 10 15))
        ;[1 0.4657 0.1578] On level 4 skeletons
        (switch `/Game/DAWID/CombatSystem/Data/EEnemyType` (`KismetArrayLibrary.Array_Random` (`local.EnemiesTypeLevel4`))
          (:`NewEnumerator4`
            ;[0.3154 1 0.3934] Skeleton
            (set `local.LevelData` (`BlueprintMapLibrary.Map_Find` (`self.Skeleton`) (`local.EnemyLvl`)))
            (set `local.Sprite` "/Game/PaperAssets/Characters/Skeleton/NoShield/FB_Skeleton_Idle_Right.FB_Skeleton_Idle_Right")
            ;[1 0.05107 0.7825] OPTIONAL
            (set `local.EnemyElement` "NONE")
            (set `local.WeaponElement` "NONE")
            (set `local.WeaponStatus` (make `CombatStatus` "NONE"))
            (set `local.StatusesImmunity` (`|MakeSet` "NONE" :!type "ECombatStatusType Enum"))
            (set `local.AnimClass` "/Game/Blueprints/Animations/Skeleton/ABP_Skeleton.ABP_Skeleton_C")
            (set `local.TakeDMGAnim` "/Game/Blueprints/Animations/Skeleton/AnimSequences/Skeleton_Hit_Right.Skeleton_Hit_Right")
            (set `local.Actions` (`|MakeArray` "/Game/DAWID/CombatSystem/Data/Actions/Skeleton/Skeleton_DefaultAttack.Skeleton_DefaultAttack_C" "/Game/DAWID/CombatSystem/Data/Actions/Skeleton/Skeleton_MultipleSlash.Skeleton_MultipleSlash_C" :!type "BLAction Soft Class Reference"))
            (set `local.Name` "Warrior")
            (goto _label_2))
          (:`NewEnumerator5`
            ;[1 0.8591 0.2111] SkeletonMage
            (set `local.LevelData` (`BlueprintMapLibrary.Map_Find` (`self.SkeletonMage`) (`local.EnemyLvl`)))
            (set `local.Sprite` "/Game/PaperAssets/Characters/SkeletonMage/NoShield/FB_SkeletonMage_Idle_Right.FB_SkeletonMage_Idle_Right")
            (set `local.EnemyElement` "NONE")
            (set `local.WeaponElement` "NONE")
            (set `local.WeaponStatus` (make `CombatStatus` "NONE"))
            (set `local.StatusesImmunity` (`|MakeSet` "NONE" :!type "ECombatStatusType Enum"))
            (set `local.AnimClass` "/Game/Blueprints/Animations/SkeletonMage/ABP_SkeletonMage.ABP_SkeletonMage_C")
            (set `local.TakeDMGAnim` "/Game/Blueprints/Animations/SkeletonMage/AnimSequences/SkeletonMage_Hit_Right.SkeletonMage_Hit_Right")
            (set `local.Actions` (`|MakeArray` "/Game/DAWID/CombatSystem/Data/Actions/SkieletonMage/SkeletonMage_DefaultAttack.SkeletonMage_DefaultAttack_C" "/Game/DAWID/CombatSystem/Data/Actions/SkieletonMage/SkeletonMage_DarkRain.SkeletonMage_DarkRain_C" "/Game/DAWID/CombatSystem/Data/Actions/SkieletonMage/SkeletonMage_BoulderRush.SkeletonMage_BoulderRush_C" :!type "BLAction Soft Class Reference"))
            (set `local.Name` "Mage")
            (goto _label_2))
          (:`NewEnumerator6`
            ;[0.4669 0.4693 1] SkeletonShield
            (set `local.LevelData` (`BlueprintMapLibrary.Map_Find` (`self.SkeletonShield`) (`local.EnemyLvl`)))
            (set `local.Sprite` "/Game/PaperAssets/Characters/Skeleton/WithShield/FB_SkeletonShield_Idle_Right.FB_SkeletonShield_Idle_Right")
            (set `local.EnemyElement` "NONE")
            (set `local.WeaponElement` "NONE")
            (set `local.WeaponStatus` (make `CombatStatus` "NONE"))
            (set `local.StatusesImmunity` (`|MakeSet` "NONE" :!type "ECombatStatusType Enum"))
            (set `local.AnimClass` "/Game/Blueprints/Animations/SkeletonShield/ABP_SkeletonShield.ABP_SkeletonShield_C")
            (set `local.TakeDMGAnim` "/Game/Blueprints/Animations/SkeletonShield/AnimSequences/SkeleotnShield_Hit_Right.SkeleotnShield_Hit_Right")
            (set `local.Actions` (`|MakeArray` "/Game/DAWID/CombatSystem/Data/Actions/SkeletonShield/SkeletonShield_DefaultAttack.SkeletonShield_DefaultAttack_C" "/Game/DAWID/CombatSystem/Data/Actions/SkeletonShield/SkeletonShield_Defend.SkeletonShield_Defend_C" :!type "BLAction Soft Class Reference"))
            (set `local.Name` "Knight")
            (goto _label_2))))
      (`BLEnemyDataAsset.SetEnemyTeamData` _combatdata_enemydata (`local.EnemyData`)))))