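; BP_PatrolEnemy is a patrolling enemy that starts combat encounters with the player.
; On BeginPlay it sets its animation and patrol speed, or destroys itself if its first tag is flagged in the game instance's enemy map.
; Normal starts (gated by CanFightMessage) and sneak attacks share a DoOnce sequence that speeds it up, optionally generates team data, shows a banner, switches AI to attack, freezes the player and triggers BPCombatComponent.
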(event `self.ReceiveBeginPlay`
  (bind _tags (`self.Tags`))
  (`parent.ReceiveBeginPlay`)
  (`KismetSystemLibrary.Delay` 0.2)
  (`PaperZDAnimationComponent.SetAnimInstanceClass` (`self.AnimationComponent`) (`self.AnimClass`))
  (bind _asbp_blgame_instance (cast `/Game/AREK/Blueprints/GameInstance/BP_BLGameInstance` (`GameplayStatics.GetGameInstance`)))
  (`/Engine/EditorBlueprintResources/StandardMacros.IsValid` _asbp_blgame_instance
    (:`Is Valid`
      (if (`KismetArrayLibrary.Array_IsNotEmpty` _tags)
        (bind (_value _returnvalue) (`BlueprintMapLibrary.Map_Find` (`BLGameInstance.GetEnemies` _asbp_blgame_instance) (`|GetArrayItem` _tags)))
        (if _returnvalue
          (if _value
            (`self.K2_DestroyActor`)
            (else
              (`self.Set Speed` false :!label _label)
              (set `self.WidgetText` "FIGHT!")))
          (else
            (goto _label)))))
    (:`Is Not Valid`
      (goto _label))))

(event `/Game/DAWID/EnemyPatrolSystem/BPI_EnemyPatrol.StartCombat`
  (params (Player :type "Actor Object Reference"))
  (if (`KismetSystemLibrary.DoesImplementInterface` Player "/Game/DAWID/EnemyPatrolSystem/BPI_Player.BPI_Player_C")
    (bind _cancombat (message `/Game/DAWID/EnemyPatrolSystem/BPI_Player.CanFight` Player))
    (if _cancombat
      (`/Engine/EditorBlueprintResources/StandardMacros.DoOnce` false :!label _label_2
        (:`Completed`
          (`self.Set Speed` true)
          (if (`self.bGenerateData`)
            (`self.GenerateEnemyTeamData`))
          (bind _returnvalue (`|CreateWidget` "/Game/DAWID/EnemyPatrolSystem/WBP_StartCombat.WBP_StartCombat_C" null (`self.WidgetText`)))
          (`UserWidget.AddToViewport` _returnvalue 0)
          (bind _asaic_patrol_enemy (cast `/Game/DAWID/EnemyPatrolSystem/AIC_PatrolEnemy` (`self.GetController`))
            (:`then`
              (`/Engine/EditorBlueprintResources/StandardMacros.IsValid` _asaic_patrol_enemy
                (:`Is Valid`
                  (`/Game/DAWID/EnemyPatrolSystem/AIC_PatrolEnemy.SetStateAsAttack` _asaic_patrol_enemy))))
            (:`CastFailed`
              _))
          (`GameplayStatics.PlaySound2D` "/Game/Audio/Combat/Background/S_StartFight.S_StartFight" 1.0 1.0 0.0 null null)
          (message `/Game/DAWID/EnemyPatrolSystem/BPI_Player.StopMovement` Player)
          (message `/Game/DAWID/EnemyPatrolSystem/BPI_Player.StartFlickering` Player)
          (`PrimitiveComponent.SetMaterial` (`self.PaperFlipbook`) 0 "/Game/AREK/Materials/MI_WhiteFlickering.MI_WhiteFlickering")
          (`BLCombatComponent.StartCombat` (`self.BP_CombatComponent`)))))))

(event `/Game/DAWID/EnemyPatrolSystem/BPI_EnemyPatrol.SneakAttack`
  (`BLCombatComponent.SneakAttack` (`self.BP_CombatComponent`))
  (set `self.WidgetText` "SNEAK ATTACK!")
  (goto _label_2))

(fn `GenerateEnemyTeamData`
  (`/Game/DAWID/CombatSystem/BP_CombatComponent.Generate Data` (`self.BP_CombatComponent`) (`self.DifficultyLevel`)))

(fn `Set Speed`
  (params (bAttack :type Boolean))
  (bind _movement (`self.Movement`))
  (if bAttack
    (set `CharacterMovementComponent.MaxWalkSpeed` 150.0 _movement)
    (else
      (set `CharacterMovementComponent.MaxWalkSpeed` 80.0 _movement))))

(fn `UserConstructionScript`
  (`parent.UserConstructionScript`))