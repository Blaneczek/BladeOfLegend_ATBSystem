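; SaveOnStart is a short-lived trigger actor that saves the game when the player overlaps it, destroying itself one second after BeginPlay.
; Overlaps on its collision component are filtered by the BPI_Player interface and limited to a single firing with DoOnce.
; The save is delegated to SaveGame on BP_BLGameInstance, followed by a debug print.
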(event `self.ReceiveBeginPlay`
  (`KismetSystemLibrary.Delay` 1.0)
  (`self.K2_DestroyActor`))

(event `self.CollisionComponent.OnComponentBeginOverlap`
  (params (OverlappedComponent :type "PrimitiveComponent Object Reference") (OtherActor :type "Actor Object Reference") (OtherComp :type "PrimitiveComponent Object Reference") (OtherBodyIndex :type Integer) (bFromSweep :type Boolean) (SweepResult :type "HitResult Structure (by ref)"))
  (if (`KismetSystemLibrary.DoesImplementInterface` OtherActor "/Game/DAWID/EnemyPatrolSystem/BPI_Player.BPI_Player_C")
    (`/Engine/EditorBlueprintResources/StandardMacros.DoOnce` false
      (:`Completed`
        (bind _asbp_blgame_instance (cast `/Game/AREK/Blueprints/GameInstance/BP_BLGameInstance` (`GameplayStatics.GetGameInstance`)))
        (`/Engine/EditorBlueprintResources/StandardMacros.IsValid` _asbp_blgame_instance
          (:`Is Valid`
            (`BLGameInstance.SaveGame` _asbp_blgame_instance)
            (`KismetSystemLibrary.PrintString` "Hasdada")))))))

(fn `UserConstructionScript`)