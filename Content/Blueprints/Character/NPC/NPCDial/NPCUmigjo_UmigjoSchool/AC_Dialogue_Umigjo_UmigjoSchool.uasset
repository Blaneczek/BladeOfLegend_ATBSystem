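; Dialogue component for the NPC Umigjo at UmigjoSchool, who offers the hero a final test of a secret technique on a mannequin.
; The Dialogue event runs DialogueContent, which selects on the active branch and shows Umigjo's speech with two replies.
; The dismissive reply adds a retort before both paths converge.
; Both close the conversation, grant Krolth_QuickSlash as a special skill to the first hero through the game instance, and signal conversation end.
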(event `self.Dialogue`
  (`self.DialogueContent`))

(fn `DialogueContent`
  (switch `name` (`self.GetActiveDialogueBranch`)
    (:`Default`
      (bind _returnvalue (`self.AddDialogue` "Your last encounter with wolves showed me you were ready to learn my secrets and I was not mistaken, there was no one who would learn my secret technique so quickly until now. As your final test I want you to execute this technique on a manequin over there." "Umigjo" (`|MakeArray` "Yea, sure, let's get this over with." "Of course, Master." :!type "Text"))
        (:`PassThrough`
          (switch `int` _returnvalue
            (:`0`
              (`self.AddDialogue` "There's no one to impress over here you know?" "Umigjo" (`|MakeArray` "Whatever..." :!type "Text")
                (:`PassThrough`
                  _)))
            (:`1`
              _))
          (`self.CloseConversation`)
          (bind _asbp_blgame_instance (cast `/Game/AREK/Blueprints/GameInstance/BP_BLGameInstance` (`GameplayStatics.GetGameInstance`)))
          (`BLGameInstance.AddSkill` _asbp_blgame_instance 0 "SPECIAL_SKILL" "/Game/DAWID/CombatSystem/Data/Actions/Krolth/Special/Krolth_QuickSlash.Krolth_QuickSlash_C")
          (`self.OnEndConverstaion`))))))