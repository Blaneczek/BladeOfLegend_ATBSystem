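; Dialogue component for Terfiyee's intro scene, a post-rescue conversation between the player, Umigjo and Terfiyee.
; The Dialogue event builds a nested AddDialogue tree, where a cocky or honest reply leads into a shared ending.
; That ending signals Terfiyee to turn back, has Umigjo summon Krolth to training, then closes the conversation and plays LS_Intro2.
; A finish callback is bound to the sequence, and a separate event opens the Umigjo school intro map.
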(event `self.Dialogue`
  (`self.DialogueContent`))

(event `OpenLevelUmigjoSchool`
  (`GameplayStatics.OpenLevel` "MAP_UmigjoSchoolIntro"))

(fn `DialogueContent`
  (switch `name` (`self.GetActiveDialogueBranch`)
    (:`Default`
      (bind _returnvalue (`self.AddDialogue` "Looks like we managed to get here in the nick of time. Ha ha ha!" "Umigjo" (`|MakeArray` "I mean.... I didn't wanna take them all myself, I wanted to leave something for you as well!" "Yeah, that was a tight one, thanks for the help." :!type "Text"))
        (:`PassThrough`
          (switch `int` _returnvalue
            (:`0`
              ;[1 1 1] Cocky
              (`self.AddDialogue` "Is this why you were running for your life without looking back?" "Umigjo" (`|MakeArray` "Huh? What? No! I wasn't...." :!type "Text")
                (:`PassThrough`
                  (`self.AddDialogue` "I appreciate the bravado, boy, but bear in mind that you have only one life, so running when there is too many enemies for you was the wise choice." "Umigjo" (`|MakeArray` "Continue" :!type "Text")
                    (:`PassThrough`
                      (`self.AddDialogue` "Well, I for one am sure glad too see no casualty on our side." "Terfiyee" (`|MakeArray` "Continue" :!type "Text")
                        (:`PassThrough`
                          (`self.AddDialogue` "Never said I didn't as well young lady." "Umigjo" (`|MakeArray` "Continue" :!type "Text")
                            (:`PassThrough`
                              _)))))))))
            (:`1`
              ;[1 1 1] Honest
              (`self.AddDialogue` "Think nothing of it, it's what we do as the militia, there were some of us more eager to run to help you out than others. Ha ha ha!" "Umigjo" (`|MakeArray` "Continue" :!type "Text")
                (:`PassThrough`
                  _))))
          (`self.OnTerfiyeeTurnBack`)
          (`self.AddDialogue` "Well, since we have done everything here, we can go back to the village. There’s no telling if we could survive a wolf horde should such appear. Krolth, you are ready for my training, report to my school once we get back.”" "Umigjo" (`|MakeArray` "Continue" :!type "Text")
            (:`PassThrough`
              (`self.CloseConversation`)
              (bind (_outactor _returnvalue_2) (`LevelSequencePlayer.CreateLevelSequencePlayer` "/Game/Cinematics/Intro2/LS_Intro2.LS_Intro2"))
              (`MovieSceneSequencePlayer.Play` _returnvalue_2)
              (add `MovieSceneSequencePlayer.OnFinished` _returnvalue_2 (`|CreateDelegate` :!event `OpenLevelUmigjoSchool`)))))))))