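; BP_NPCTerfiyee_Intro0 is the Terfiyee NPC variant for an intro dialogue, built on an inherited NPC base with animation, dialogue and Paper2D flipbook components.
; Shortly after BeginPlay, it assigns the ABP_Terfiyee anim instance and casts its dialogue component to AC_Dialogue_Terfiyee_Intro0.
; It binds to that component's OnTerfiyeeTurnBack event, which switches the flipbook to the right-facing idle.
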(event `self.ReceiveBeginPlay`
  (`parent.ReceiveBeginPlay`)
  (`KismetSystemLibrary.Delay` 0.3)
  (`PaperZDAnimationComponent.SetAnimInstanceClass` (`self.AnimationComponent`) "/Game/Blueprints/Animations/Terfiyee/ABP_Terfiyee.ABP_Terfiyee_C")
  (bind _asac_dialogue_terfiyee_intro_0 (cast `/Game/Blueprints/Character/NPC/NPCDial/NPCTerfiyee_Intro0/AC_Dialogue_Terfiyee_Intro0` (`self.DialogueComponent`)))
  (add `/Game/Blueprints/Character/NPC/NPCDial/NPCTerfiyee_Intro0/AC_Dialogue_Terfiyee_Intro0.OnTerfiyeeTurnBack` _asac_dialogue_terfiyee_intro_0 (delegate `CustomEvent`)))

(event `CustomEvent`
  (`PaperFlipbookComponent.SetFlipbook` (`self.PaperFlipbook`) "/Game/PaperAssets/Characters/Terfiyee/FB_Terfiyee_Idle_Right.FB_Terfiyee_Idle_Right"))

(fn `UserConstructionScript`
  (`parent.UserConstructionScript`))