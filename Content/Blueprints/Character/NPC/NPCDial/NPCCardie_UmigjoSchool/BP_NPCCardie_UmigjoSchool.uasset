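; BP_NPCCardie_UmigjoSchool is the Cardie NPC for UmigjoSchool, who appears through dialogue and is added as a hero afterward.
; BeginPlay sets the Cardie animation class, then binds to two events on its Cardie-specific dialogue component.
; OnShowCardie makes the sprite visible with a left-facing idle flipbook.
; OnEndConvo adds Cardie's asset info to the game instance, re-enables player input and prints a debug string.
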(event `self.ReceiveBeginPlay`
  (`parent.ReceiveBeginPlay`)
  (`PaperZDAnimationComponent.SetAnimInstanceClass` (`self.AnimationComponent`) "/Game/Blueprints/Animations/Cardie/ABP_Cardie.ABP_Cardie_C")
  (bind _asac_dialogue_cardie_umigjo_school (cast `/Game/Blueprints/Character/NPC/NPCDial/NPCCardie_UmigjoSchool/AC_Dialogue_Cardie_UmigjoSchool` (`self.DialogueComponent`)))
  (bind _output_get (set `self.CardieDialogueComponent` _asac_dialogue_cardie_umigjo_school))
  (add `/Game/Blueprints/Character/NPC/NPCDial/NPCCardie_UmigjoSchool/AC_Dialogue_Cardie_UmigjoSchool.OnShowCardie` _output_get (delegate `OnShowCardie_Event`))
  (add `/Game/Blueprints/Character/NPC/NPCDial/NPCCardie_UmigjoSchool/AC_Dialogue_Cardie_UmigjoSchool.OnEndConvo` (`self.CardieDialogueComponent`) (delegate `OnEndConvo_Event`)))

(event `OnShowCardie_Event`
  (`SceneComponent.SetVisibility` (`self.Sprite`) true false)
  (`PaperFlipbookComponent.SetFlipbook` (`self.PaperFlipbook`) "/Game/PaperAssets/Characters/Cardie/FB_Cardie_Idle_Left.FB_Cardie_Idle_Left"))

(event `OnEndConvo_Event`
  (bind _asbp_blgame_instance (cast `/Game/AREK/Blueprints/GameInstance/BP_BLGameInstance` (`GameplayStatics.GetGameInstance`)))
  (`BLGameInstance.AddHero` _asbp_blgame_instance (`self.CardieAssetInfo`))
  (`self.EnableInput` (`GameplayStatics.GetPlayerCharacter` 0) (`GameplayStatics.GetPlayerController` 0))
  (`KismetSystemLibrary.PrintString` "cardie"))

(fn `UserConstructionScript`
  (`parent.UserConstructionScript`))