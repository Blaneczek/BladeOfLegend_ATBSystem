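; Dialogue component for the Umigjo school scene, in which Umigjo introduces his magic student Cardie and sends her and Krolth to investigate the wolf uproar.
; The Dialogue event runs DialogueContent, a linear chain of AddDialogue calls with a single response each, alternating between Umigjo and Cardie.
; CallOnShowCardie fires before Cardie's first line.
; The final response fires CallOnEndConvo and closes the conversation.
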(event `self.Dialogue`
  (`self.DialogueContent`))

(fn `DialogueContent`
  (switch `name` (`self.GetActiveDialogueBranch`)
    (:`Default`
      (`self.AddDialogue` "Well done my student, your training with me has paid off." "Umigjo" (`|MakeArray` "Continue" :!type "Text")
        (:`PassThrough`
          (`self.AddDialogue` "Now there is much I can still teach you, but for that you need to get stronger and I have to see that you wield a better weapon." "Umigjo" (`|MakeArray` "All right, I’m going out to train on my own now, militia will appreciate my newfound strength." :!type "Text")
            (:`PassThrough`
              (`self.AddDialogue` "Good to see you’re full of vigor to learn more. Now I have a task for you that you should be to handle now." "Umigjo" (`|MakeArray` "A task?" :!type "Text")
                (:`PassThrough`
                  (`self.AddDialogue` "Yes, as you’ve noticed for yourself, the wolf population has grown much more violent and with your newfound skill you should be able to handle more of them now, that’s why I would like you to cooperate with my magic arts student, Cardie" "Umigjo" (`|MakeArray` "I didn’t know you taught magic as well master Umigjo." :!type "Text")
                    (:`PassThrough`
                      (`self.AddDialogue` "You did not ask for magic lessons, so I did not give any, but there are more important things now." "Umigjo" (`|MakeArray` "Continue" :!type "Text")
                        (:`PassThrough`
                          (`self.OnShowCardie`)
                          (`self.AddDialogue` "Hello master Umigjo, you called for me?" "Cardie" (`|MakeArray` "Continue" :!type "Text")
                            (:`PassThrough`
                              (`self.AddDialogue` "Ah Cardie, I was just talking about you, yes I have requested your presence. I would like you to cooperate with Krolth to \ninvestigate and hopefully put a stop to the wolf uproar. Both of you should be strong enough to handle it if you cooperate. \n" "Umigjo" (`|MakeArray` "I'm grateful for the opportunity to work together." :!type "Text")
                                (:`PassThrough`
                                  (`self.AddDialogue` "Oh my, a flatterer, master hold me or I'll get a jump on him\"." "Cardie" (`|MakeArray` "Continue" :!type "Text")
                                    (:`PassThrough`
                                      (`self.AddDialogue` "Cardie, this is no joking matter." "Umigjo" (`|MakeArray` "Continue" :!type "Text")
                                        (:`PassThrough`
                                          (`self.AddDialogue` "Sorry, sorry, anyway, nice to meet you too handsome." "Cardie" (`|MakeArray` "Continue" :!type "Text")
                                            (:`PassThrough`
                                              (`self.AddDialogue` "Before you go, I have crystals for you that will enhance your abilities. However, you cannot use them without first saturating the crystals. Find the Crystal Binder; it’s in the village. Thanks to it, you will be stronger." "Umigjo" (`|MakeArray` "Continue" :!type "Text")
                                                (:`PassThrough`
                                                  (`self.AddDialogue` "Now with that out of the way, I'll give you a few items that you can also buy in the village once you run out of them." "Umigjo" (`|MakeArray` "Continue" :!type "Text")
                                                    (:`PassThrough`
                                                      (`self.AddDialogue` "Thank you master. \n(To Krolth) Shall we?" "Cardie" (`|MakeArray` "Yeah, let's go." :!type "Text")
                                                        (:`PassThrough`
                                                          (`self.OnEndConvo`)
                                                          (`self.CloseConversation`))))))))))))))))))))))))))))))