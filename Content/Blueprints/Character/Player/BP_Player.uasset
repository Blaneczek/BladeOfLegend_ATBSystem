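; BP_Player is the Paper2D player character Krolth for exploration, handling sneak attacks on patrolling enemies and the menu toggle.
; BeginPlay shows the end-game widget or restores post-combat or saved location from BP_BLGameInstance, and adds companions.
; An Attack overlap tracks the enemy, and IA_Attack plays a directional animation override, then sends it SneakAttackMessage.
; A landed sneak attack locks input, clears CanFight and applies a white flicker material; U triggers LevelUP.
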(event `Key|U`
  (params (Key :type "Key Structure"))
  (:`Pressed`
    (bind _asbp_blgame_instance (cast `/Game/AREK/Blueprints/GameInstance/BP_BLGameInstance` (`GameplayStatics.GetGameInstance`)))
    (`BLGameInstance.LevelUP` _asbp_blgame_instance)))

(event `Key|K`
  (params (Key :type "Key Structure")))

(event `self.ReceiveBeginPlay`
  (`|ExecutionSequence`
    (:`then_0`
      (`parent.ReceiveBeginPlay`)
      (`WidgetBlueprintLibrary.SetInputMode_GameOnly` (`GameplayStatics.GetPlayerController` 0))
      (bind _asbp_blgame_instance (cast `/Game/AREK/Blueprints/GameInstance/BP_BLGameInstance` (`GameplayStatics.GetGameInstance`)))
      (set `self.GameInstance` _asbp_blgame_instance)
      (if (`BLGameInstance.IsEndGame` (`self.GameInstance`))
        (bind _returnvalue (`|CreateWidget` "/Game/UI/EndGame/WBP_EndGame.WBP_EndGame_C"))
        (`UserWidget.AddToViewport` _returnvalue 0)
        (elif (`BLGameInstance.UseCombatPlayerLocation` (`self.GameInstance`))
          (`self.K2_SetActorLocation` (`BLGameInstance.GetNewPostCombatLocation` (`self.GameInstance`)))
          (`BLGameInstance.SetUseCombatPlayerLocation` (`self.GameInstance`) false)
          (elif (`BLGameInstance.UseSavedPlayerLocation` (`self.GameInstance`))
            (`self.K2_SetActorLocation` (`BLGameInstance.GetSavedLocation` (`self.GameInstance`)))
            (`BLGameInstance.SetUseSavedPlayerLocation` (`self.GameInstance`) false)))))
    (:`then_1`
      (`self.AddCompanions`)
      (`KismetSystemLibrary.Delay` 0.2)
      (`PaperZDAnimationComponent.SetAnimInstanceClass` (`self.AnimationComponent`) "/Game/Blueprints/Animations/Krolth/ABP_Krolth.ABP_Krolth_C"))))

(event `/Game/DAWID/EnemyPatrolSystem/BPI_Player.StartFlickering`
  ;[1 1 1] When starting fight with enemy
  (set `self.bCanFight` false)
  (`PrimitiveComponent.SetMaterial` (`self.PaperFlipbook`) 0 "/Game/AREK/Materials/MI_WhiteFlickering.MI_WhiteFlickering"))

(event `/Game/DAWID/EnemyPatrolSystem/BPI_Player.StopMovement`
  ;[1 1 1] When starting fight with enemy
  (`self.DisableInput` (`GameplayStatics.GetPlayerController` 0)))

(event `EnhancedInput|/Game/AREK/Input/Actions/IA_Attack`
  (params (ActionValue :type Boolean) (ElapsedSeconds :type "Float (double-precision)") (TriggeredSeconds :type "Float (double-precision)") (InputAction :type "InputAction Object Reference" :default "/Game/AREK/Input/Actions/IA_Attack.IA_Attack"))
  (bind _returnvalue_x (`KismetMathLibrary.BreakVector` (`self.GetActorForwardVector`)))
  ;[1 1 1] Sneak attack
  (:`Started`
    (`self.DisableInput` (`GameplayStatics.GetPlayerController` 0))
    (if (> _returnvalue_x 0.0)
      (`self.EnemyActor`
        (:`then`
          (`PaperZDPlaySlotOverrideAction.PlayAnimationOverrideWithCallbacks` (`PaperZDAnimationComponent.AnimInstance` (`self.AnimationComponent`)) "/Game/Blueprints/Animations/Krolth/AnimSequences/Krolth_Attack1_Right.Krolth_Attack1_Right"
            (:`OnCompleted`
              _)
            (:`OnCancelled`
              _)))
        (:`else`
          (`PaperZDPlaySlotOverrideAction.PlayAnimationOverrideWithCallbacks` (`PaperZDAnimationComponent.AnimInstance` (`self.AnimationComponent`)) "/Game/Blueprints/Animations/Krolth/AnimSequences/Krolth_Attack1_Right1.Krolth_Attack1_Right1"
            (:`OnCompleted`
              _)
            (:`OnCancelled`
              _))))
      (else
        (`self.EnemyActor`
          (:`then`
            (`PaperZDPlaySlotOverrideAction.PlayAnimationOverrideWithCallbacks` (`PaperZDAnimationComponent.AnimInstance` (`self.AnimationComponent`)) "/Game/Blueprints/Animations/Krolth/AnimSequences/Krolth_Attack1_Left.Krolth_Attack1_Left"
              (:`OnCompleted`
                _)
              (:`OnCancelled`
                _)))
          (:`else`
            (`PaperZDPlaySlotOverrideAction.PlayAnimationOverrideWithCallbacks` (`PaperZDAnimationComponent.AnimInstance` (`self.AnimationComponent`)) "/Game/Blueprints/Animations/Krolth/AnimSequences/Krolth_Attack1_Left1.Krolth_Attack1_Left1"
              (:`OnCompleted`
                _)
              (:`OnCancelled`
                _))))))
    (`self.EnableInput` (`GameplayStatics.GetPlayerController` 0))
    (bind _enemyactor (`self.EnemyActor`)
      (:`then`
        (`KismetSystemLibrary.PrintString` "Sneak attack")
        (message `/Game/DAWID/EnemyPatrolSystem/BPI_EnemyPatrol.SneakAttack` _enemyactor)
        (`self.StopMovement`)
        (`self.StartFlickering`))
      (:`else`
        (`KismetSystemLibrary.PrintString` "used attack")))))

(event `self.Attack.OnComponentBeginOverlap`
  (params (OverlappedComponent :type "PrimitiveComponent Object Reference") (OtherActor :type "Actor Object Reference") (OtherComp :type "PrimitiveComponent Object Reference") (OtherBodyIndex :type Integer) (bFromSweep :type Boolean) (SweepResult :type "HitResult Structure (by ref)"))
  ;[1 1 1] Sneak attack
  (if (`KismetSystemLibrary.DoesImplementInterface` OtherActor "/Game/DAWID/EnemyPatrolSystem/BPI_EnemyPatrol.BPI_EnemyPatrol_C")
    (set `self.EnemyActor` OtherActor)))

(event `self.Attack.OnComponentEndOverlap`
  (params (OverlappedComponent :type "PrimitiveComponent Object Reference") (OtherActor :type "Actor Object Reference") (OtherComp :type "PrimitiveComponent Object Reference") (OtherBodyIndex :type Integer))
  ;[1 1 1] Sneak attack
  (if (== OtherActor (`self.EnemyActor`))
    (set `self.EnemyActor` null)))

(event `EnhancedInput|/Game/AREK/Input/Actions/IA_Interface`
  (params (ActionValue :type Boolean) (ElapsedSeconds :type "Float (double-precision)") (TriggeredSeconds :type "Float (double-precision)") (InputAction :type "InputAction Object Reference" :default "/Game/AREK/Input/Actions/IA_Interface.IA_Interface"))
  (:`Completed`
    (`/Engine/EditorBlueprintResources/StandardMacros.IsValid` (`self.WBP_InterfaceRef`)
      (:`Is Valid`
        _)
      (:`Is Not Valid`
        (bind _returnvalue (`|CreateWidget` "/Game/UI/Interface/MainScreen/WBP_Interface.WBP_Interface_C"))
        (set `self.WBP_InterfaceRef` _returnvalue)))
    (`BLInterfaceWidget.ToggleMenu` (`self.WBP_InterfaceRef`))))

(fn `CanFight`
  (returns (CanCombat :type Boolean))
  (return (`self.bCanFight`)))

(fn `UserConstructionScript`)