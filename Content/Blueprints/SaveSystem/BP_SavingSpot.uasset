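; BP_SavingSpot is a save point that saves the game when a BPI_Player actor overlaps its box.
; BeginPlay animates the opacity of four hieroglyph sprites, then enables saving.
; A DoOnce-gated overlap calls SaveGame on BP_BLGameInstance, shows WBP_SaveGame and plays a second opacity timeline.
; After the player leaves, a delayed Reset plays a third timeline and re-arms the DoOnce.
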(event `self.ReceiveBeginPlay`
  (set `self.bCanSave` false)
  (bind (_direction _opacity) (`Timeline|Timeline` :!via `PlayFromStart`)
    (:`Update`
      (`PaperSpriteComponent.SetSpriteColor` (`self.Hieroglyph3`) (make `LinearColor` 0.0 0.596179 0.830209 _opacity))
      (`PaperSpriteComponent.SetSpriteColor` (`self.Hieroglyph2`) (make `LinearColor` 0.0 0.596179 0.830209 _opacity))
      (`PaperSpriteComponent.SetSpriteColor` (`self.Hieroglyph1`) (make `LinearColor` 0.0 0.596179 0.830209 _opacity))
      (`PaperSpriteComponent.SetSpriteColor` (`self.Hieroglyph0`) (make `LinearColor` 0.0 0.596179 0.830209 _opacity)))
    (:`Finished`
      (set `self.bCanSave` true))))

(event `self.Box.OnComponentBeginOverlap`
  (params (OverlappedComponent :type "PrimitiveComponent Object Reference") (OtherActor :type "Actor Object Reference") (OtherComp :type "PrimitiveComponent Object Reference") (OtherBodyIndex :type Integer) (bFromSweep :type Boolean) (SweepResult :type "HitResult Structure (by ref)"))
  (`KismetSystemLibrary.PrintString` "Hello")
  (if (`self.bCanSave`)
    (if (`KismetSystemLibrary.DoesImplementInterface` OtherActor "/Game/DAWID/EnemyPatrolSystem/BPI_Player.BPI_Player_C")
      (`/Engine/EditorBlueprintResources/StandardMacros.DoOnce` false :!label _label
        (:`Completed`
          (bind _asbp_blgame_instance (cast `/Game/AREK/Blueprints/GameInstance/BP_BLGameInstance` (`GameplayStatics.GetGameInstance`)))
          (`/Engine/EditorBlueprintResources/StandardMacros.IsValid` _asbp_blgame_instance
            (:`Is Valid`
              (set `self.bSaved` true)
              (`BLGameInstance.SaveGame` _asbp_blgame_instance)
              (bind _returnvalue (`|CreateWidget` "/Game/UI/WBP_SaveGame.WBP_SaveGame_C"))
              (`UserWidget.AddToViewport` _returnvalue 0)
              (bind (_direction _opacity) (`Timeline|Timeline_0` :!via `PlayFromStart`)
                (:`Update`
                  (`PaperSpriteComponent.SetSpriteColor` (`self.Hieroglyph3`) (make `LinearColor` 0.0 0.596179 0.830209 _opacity))
                  (`PaperSpriteComponent.SetSpriteColor` (`self.Hieroglyph2`) (make `LinearColor` 0.0 0.596179 0.830209 _opacity))
                  (`PaperSpriteComponent.SetSpriteColor` (`self.Hieroglyph1`) (make `LinearColor` 0.0 0.596179 0.830209 _opacity))
                  (`PaperSpriteComponent.SetSpriteColor` (`self.Hieroglyph0`) (make `LinearColor` 0.0 0.596179 0.830209 _opacity)))))))))))

(event `self.Box.OnComponentEndOverlap`
  (params (OverlappedComponent :type "PrimitiveComponent Object Reference") (OtherActor :type "Actor Object Reference") (OtherComp :type "PrimitiveComponent Object Reference") (OtherBodyIndex :type Integer))
  (if (`self.bSaved`)
    (if (`KismetSystemLibrary.DoesImplementInterface` OtherActor "/Game/DAWID/EnemyPatrolSystem/BPI_Player.BPI_Player_C")
      (set `self.bSaved` false)
      (`KismetSystemLibrary.K2_SetTimerDelegate` (delegate `Reset`) 5.0))))

(event `Reset`
  (bind (_direction _opacity) (`Timeline|Timeline_1` :!via `PlayFromStart`)
    (:`Update`
      (`PaperSpriteComponent.SetSpriteColor` (`self.Hieroglyph3`) (make `LinearColor` 0.0 0.596179 0.830209 _opacity))
      (`PaperSpriteComponent.SetSpriteColor` (`self.Hieroglyph2`) (make `LinearColor` 0.0 0.596179 0.830209 _opacity))
      (`PaperSpriteComponent.SetSpriteColor` (`self.Hieroglyph1`) (make `LinearColor` 0.0 0.596179 0.830209 _opacity))
      (`PaperSpriteComponent.SetSpriteColor` (`self.Hieroglyph0`) (make `LinearColor` 0.0 0.596179 0.830209 _opacity)))
    (:`Finished`
      (goto _label :!via `Reset`))))

(fn `UserConstructionScript`)